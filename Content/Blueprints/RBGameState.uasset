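; Game state Blueprint that keeps the Red and Blue team rosters of player states.
; UpdateTeam casts the given player to RBPlayerState and reads its Team enum to choose a roster.
; It adds the player to that roster if absent and removes them from the other, with any value but the first enum entry counting as Blue.
; The event graph and construction script are empty.
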(event EventBeginPlay)

(event EventTick
  (params (DeltaSeconds :type Float%20%28single-precision%29)))

(fn ConstructionScript)

(fn UpdateTeam
  (params (Player :type Player%20State%20Object%20Reference))
  (bind _redteam (Variables|Default|GetRedTeam))
  (bind _blueteam (Variables|Default|GetBlueTeam))
  (bind _asrbplayer_state (Utilities|Casting|CastToRBPlayerState Player))
  (if (Utilities|Enum|Equal(Enum) (Variables|/Game/Blueprints/RBPlayerState.RBPlayerState_C|GetTeam _asrbplayer_state) "NewEnumerator0")
    (if (not (Utilities|Array|ContainsItem _redteam _asrbplayer_state))
      (Utilities|Array|Add _redteam _asrbplayer_state)
      (Utilities|Array|RemoveItem _blueteam _asrbplayer_state))
    (elif (not (Utilities|Array|ContainsItem _blueteam _asrbplayer_state))
      (Utilities|Array|Add _blueteam _asrbplayer_state)
      (Utilities|Array|RemoveItem _redteam _asrbplayer_state))))