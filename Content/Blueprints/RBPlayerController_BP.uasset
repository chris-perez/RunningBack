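; Player controller for the RunningBack game that manages pawn spawning, respawning and the player's UI.
; Respawning, also bound to R, kills pawn and weapon, runs a looping-timer countdown widget, then possesses a new pawn at a GameMode-chosen spawn, updating PlayerState.
; Tick stops the pawn while GameState is Starting Game.
; It lazily creates HUD, lobby, pause (P) and scoreboard (Tab) widgets, the latter two only once the game has started.
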(event Custom|UpdateTimeToStart
  (bind _returnvalue (Math|DateTime|Now))
  (bind _timerstart (Variables|Default|GetTimerStart))
  (bind _respawntime (Variables|Default|GetRespawnTime))
  (bind _returnvalue_2 (- _returnvalue _timerstart))
  (bind _returnvalue_3 (Math|Timespan|GetSeconds _returnvalue_2))
  (bind _returnvalue_4 (- _respawntime _returnvalue_3))
  ;[1 1 1] Start Timer
  (bind _asrbplayer_controller_bp (Utilities|Casting|CastToRBPlayerController_BP (Game|GetPlayerController 0)))
  (CallFunction|DisplayCountdown _asrbplayer_controller_bp _returnvalue_4)
  (if (<= _returnvalue_4 0)
    (Class|KismetSystemLibrary|ClearTimerHandle (stale Custom|RespawnDelayed _returnvalue))
    (Utilities|IsValid (Variables|RBPlayerController_BP_C|GetCountdownWidget _asrbplayer_controller_bp)
      (:Is%20Valid
        (Widget|RemovefromParent (Variables|RBPlayerController_BP_C|GetCountdownWidget _asrbplayer_controller_bp))
        (Variables|RBPlayerController_BP_C|SetCountdownWidget _asrbplayer_controller_bp 0)
        (CallFunction|Respawn)))))

(event Custom|Respawn
  ;[1 1 1] Kill actor and respawn at new random spawn
  (CallFunction|KillPawn)
  (CallFunction|SpawnPawn)
  (CallFunction|AllowMovement))

(event Custom|Kill%20Pawn
  (bind _returnvalue (Pawn|GetControlledPawn))
  ;[1 1 1] Kill Pawn
  (Utilities|IsValid _returnvalue
    (:Is%20Valid
      (bind _asrunning_back_pawn_bp (Utilities|Casting|CastToRunningBackPawn_BP _returnvalue))
      (Actor|DestroyActor (Variables|/Script/RunningBack.RunningBackPawn|GetSpawnedWeapon _asrunning_back_pawn_bp))
      (Actor|DestroyActor _returnvalue))))

(event Custom|CreateHUD
  ;[1 1 1] Display HUD
  (Development|PrintString "Create HUD" false true "(R=1.000000,G=0.997031,B=0.305378,A=1.000000)" 5.0)
  (Utilities|IsValid (Variables|Default|GetHUD)
    (:Is%20Valid
      _)
    (:Is%20Not%20Valid
      (bind _returnvalue (UserInterface|CreateWidget "/Game/UI/HUD.HUD_C" self))
      (Variables|Default|SetHUD _returnvalue)))
  (UserInterface|Viewport|AddtoViewport (Variables|Default|GetHUD) 0))

(event Custom|Remove%20Lobby%20Widget
  (bind _lobbymenu (Variables|Default|GetLobbyMenu))
  ;[1 1 1] Remove Lobby Widget
  (Utilities|IsValid _lobbymenu
    (:Is%20Valid
      (Widget|RemovefromParent _lobbymenu))))

(event Custom|Spawn%20Pawn
  (bind _self self)
  ;[1 1 1] Spawn Pawn
  (bind _asrbgame_mode_bp (Utilities|Casting|CastToRBGameMode_BP (Game|GetGameMode)))
  (bind _returnvalue (Default|GetSpawn _asrbgame_mode_bp _self))
  (bind _returnvalue_2 (Game|SpawnActorfromClass "/Game/Blueprints/Pawn/RunningBackPawn_BP.RunningBackPawn_BP_C" (Transformation|GetActorTransform _returnvalue) "Undefined" _self 0))
  (Pawn|Possess _returnvalue_2)
  (bind _asrbplayer_state_bp (Utilities|Casting|CastToRBPlayerState_BP (Variables|Default|GetPlayerState)))
  (Variables|/Game/Blueprints/RBPlayerState_BP.RBPlayerState_BP_C|SetState _asrbplayer_state_bp "NewEnumerator0"))

(event Custom|Update%20Lobby%20Widget)

(event Custom|Display%20Lobby%20Widget
  ;[1 1 1] Display Lobby Widget
  (Utilities|IsValid (Variables|Default|GetLobbyMenu)
    (:Is%20Valid
      _)
    (:Is%20Not%20Valid
      (bind _returnvalue (UserInterface|CreateWidget "/Game/UI/GameLobby.GameLobby_C" (Game|GetPlayerController 0)))
      (Variables|Default|SetLobbyMenu _returnvalue)))
  (UserInterface|Viewport|AddtoViewport (Variables|Default|GetLobbyMenu) 0))

(event Custom|DisplayCountdown
  (params (Time :type Integer))
  ;[1 1 1] Countdown
  ;[1 1 1] This Fixed IT
  (Input|SetInputModeGameOnly self)
  (Class|WidgetBlueprintLibrary|SetFocustoGameViewport)
  (Utilities|IsValid (Variables|Default|GetCountdownWidget)
    (:Is%20Valid
      _)
    (:Is%20Not%20Valid
      (bind _returnvalue (UserInterface|CreateWidget "/Game/UI/Countdown.Countdown_C" self))
      (Variables|Default|SetCountdownWidget _returnvalue)
      (UserInterface|Viewport|AddtoViewport (Variables|Default|GetCountdownWidget) 0)))
  (Default|SetTime (Variables|Default|GetCountdownWidget) Time))

(event Custom|RespawnDelayed
  ;[1 1 1] Start Timer
  (CallFunction|KillPawn)
  (bind _asrbplayer_state_bp (Utilities|Casting|CastToRBPlayerState_BP (Variables|Default|GetPlayerState)))
  (Variables|/Game/Blueprints/RBPlayerState_BP.RBPlayerState_BP_C|SetState _asrbplayer_state_bp "NewEnumerator2")
  (Variables|Default|SetTimerStart (Math|DateTime|Now))
  (bind _returnvalue (Utilities|Time|SetTimerbyEvent (delegate Custom|UpdateTimeToStart) 1.0 true)))

(event EventBeginPlay
  (Variables|Default|SetbShowMouseCursor false))

(event EventTick
  (params (DeltaSeconds :type Float%20%28single-precision%29))
  ;[1 1 1] Tick
  (bind _asrbgame_state_bp (Utilities|Casting|CastToRBGameState_BP (Game|GetGameState)))
  (Utilities|IsValid _asrbgame_state_bp
    (:Is%20Valid
      (switch Utilities|FlowControl|Switch|SwitchonStateOfGame (Variables|/Game/Blueprints/RBGameState_BP.RBGameState_BP_C|GetState _asrbgame_state_bp)
        (:NewEnumerator8
          (CallFunction|KeepfromMoving))))))

(event Input|KeyboardEvents|P
  (params (Key :type Key%20Structure :default "AnyKey"))
  ;[1 1 1] Pause Menu
  (:Pressed
    ;;[1 1 1] Tab and Pause only work if in game.
    (bind _asrbgame_state_bp (Utilities|Casting|CastToRBGameState_BP (Game|GetGameState)))
    (if (Variables|/Game/Blueprints/RBGameState_BP.RBGameState_BP_C|GetStarted _asrbgame_state_bp)
      (Utilities|IsValid (Variables|Default|GetPauseMenu)
        (:Is%20Valid
          _)
        (:Is%20Not%20Valid
          (bind _returnvalue (UserInterface|CreateWidget "/Game/UI/PauseMenu.PauseMenu_C"))
          (Variables|Default|SetPauseMenu _returnvalue)))
      (Input|SetInputModeUIOnly (Game|GetPlayerController 0) (Variables|Default|GetPauseMenu) false)
      (UserInterface|Viewport|AddtoViewport (Variables|Default|GetPauseMenu) 0))))

(event Input|KeyboardEvents|F
  (params (Key :type Key%20Structure :default "AnyKey")))

(event Input|KeyboardEvents|R
  (params (Key :type Key%20Structure :default "AnyKey"))
  ;[1 1 1] Manual Respawn
  (:Pressed
    (CallFunction|RespawnDelayed)))

(event Input|KeyboardEvents|G
  (params (Key :type Key%20Structure :default "AnyKey")))

(event Input|KeyboardEvents|Tab
  (params (Key :type Key%20Structure :default "AnyKey"))
  ;[1 1 1] Tab Menu
  (:Pressed
    ;;[1 1 1] Tab and Pause only work if in game.
    (bind _asrbgame_state_bp (Utilities|Casting|CastToRBGameState_BP (Game|GetGameState)))
    (if (Variables|/Game/Blueprints/RBGameState_BP.RBGameState_BP_C|GetStarted _asrbgame_state_bp)
      (Utilities|IsValid (Variables|Default|GetTabMenu)
        (:Is%20Valid
          _)
        (:Is%20Not%20Valid
          (bind _returnvalue (UserInterface|CreateWidget "/Game/UI/Scoreboard.Scoreboard_C" (Game|GetPlayerController 0)))
          (Variables|Default|SetTabMenu _returnvalue)))
      (UserInterface|Viewport|AddtoViewport (Variables|Default|GetTabMenu) 0)))
  (:Released
    (Utilities|IsValid (Variables|Default|GetTabMenu)
      (:Is%20Valid
        (Widget|RemovefromParent (Variables|Default|GetTabMenu))))))

(fn ConstructionScript)

(fn KeepfromMoving
  ;[1 1 1] Keep car from moving while not playing
  (bind _asrunning_back_pawn_bp (Utilities|Casting|CastToRunningBackPawn_BP (Pawn|GetControlledPawn)))
  (Default|SetStop _asrunning_back_pawn_bp true))

(fn AllowMovement
  ;[1 1 1] Keep car from moving while not playing
  (bind _asrunning_back_pawn_bp (Utilities|Casting|CastToRunningBackPawn_BP (Pawn|GetControlledPawn)))
  (Default|SetStop _asrunning_back_pawn_bp false))