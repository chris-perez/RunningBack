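; Game state Blueprint that keeps Red and Blue team rosters and their scores.
; RefreshTeams rebuilds both rosters from the PlayerArray using each RBPlayerState's Team value.
; UpdateTeam places a single player on the matching roster and removes them from the other.
; UpdateScore recomputes each team's score by summing its members' Points.
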(event Custom|Refresh%20Teams
  (Utilities|Array|Clear (Variables|Default|GetRedTeam))
  (Utilities|Array|Clear (Variables|Default|GetBlueTeam))
  (for _array_element (Variables|Default|GetPlayerArray)
    (bind _asrbplayer_state (Utilities|Casting|CastToRBPlayerState _array_element))
    (if (Utilities|Enum|Equal(Enum) (Variables|/Game/Blueprints/RBPlayerState.RBPlayerState_C|GetTeam _asrbplayer_state) "NewEnumerator0")
      (Utilities|Array|Add (Variables|Default|GetRedTeam) _asrbplayer_state)
      (else
        (Utilities|Array|Add (Variables|Default|GetBlueTeam) _asrbplayer_state)))))

(event EventBeginPlay)

(event EventTick
  (params (DeltaSeconds :type Float%20%28single-precision%29)))

(fn ConstructionScript)

(fn UpdateTeam
  (params (Player :type Player%20State%20Object%20Reference))
  (bind _redteam (Variables|Default|GetRedTeam))
  (bind _blueteam (Variables|Default|GetBlueTeam))
  (bind _asrbplayer_state (Utilities|Casting|CastToRBPlayerState Player))
  (if (Utilities|Enum|Equal(Enum) (Variables|/Game/Blueprints/RBPlayerState.RBPlayerState_C|GetTeam _asrbplayer_state) "NewEnumerator0")
    (if (not (Utilities|Array|ContainsItem _redteam _asrbplayer_state))
      (Utilities|Array|Add _redteam _asrbplayer_state)
      (Utilities|Array|RemoveItem _blueteam _asrbplayer_state))
    (elif (not (Utilities|Array|ContainsItem _blueteam _asrbplayer_state))
      (Utilities|Array|Add _blueteam _asrbplayer_state)
      (Utilities|Array|RemoveItem _redteam _asrbplayer_state))))

(fn UpdateScore
  (Variables|Default|SetRedScore 0)
  (for _array_element (Variables|Default|GetRedTeam)
    (bind _asrbplayer_state (Utilities|Casting|CastToRBPlayerState _array_element))
    (Variables|Default|SetRedScore (+ (Variables|Default|GetRedScore) (Variables|/Game/Blueprints/RBPlayerState.RBPlayerState_C|GetPoints _asrbplayer_state))))
  (Variables|Default|SetBlueScore 0)
  (for _array_element_2 (Variables|Default|GetBlueTeam)
    (bind _asrbplayer_state_2 (Utilities|Casting|CastToRBPlayerState _array_element_2))
    (Variables|Default|SetBlueScore (+ (Variables|Default|GetBlueScore) (Variables|/Game/Blueprints/RBPlayerState.RBPlayerState_C|GetPoints _asrbplayer_state_2)))))