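; Pickup actor for weapons and power-ups: turret gun, lazer gun, freeze ray, missile, bubble shield and drone.
; The construction script switches on the Type variable and adds static mesh components with per-type offset, rotation and scale, so each variant gets its own look.
; The drone is built from two meshes with composed transforms.
; The event graph holds only disabled placeholder events, with no overlap or collection logic.
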(event EventBeginPlay)

(event EventActorBeginOverlap
  (params (OtherActor :type Actor%20Object%20Reference)))

(event EventTick
  (params (DeltaSeconds :type Float%20%28single-precision%29)))

(fn ConstructionScript
  (bind _returnvalue (Math|Transform|MakeTransform "0.000000,0.000000,0.000000" "0.000000, 0,0.000000" "1.000000,1.000000,1.000000"))
  (bind _returnvalue_2 (Math|Transform|MakeTransform "0, 0, 0" "0, 0, 0" "4.000000,4.000000,4.000000"))
  (switch Utilities|FlowControl|Switch|SwitchonPickupType (Variables|Default|GetType)
    (:NewEnumerator0
      (AddComponent|AddStaticMeshComponent false (Math|Transform|MakeTransform "-40.000000,-50.000000,40.000000" "0.000000, 0,90.000000" "0.750000,0.750000,0.750000")))
    (:NewEnumerator1
      (AddComponent|AddStaticMeshComponent false _returnvalue_2))
    (:NewEnumerator2
      (AddComponent|AddStaticMeshComponent false _returnvalue_2))
    (:NewEnumerator3
      (AddComponent|AddStaticMeshComponent false (Math|Transform|MakeTransform "-170.000000,0.000000,-100.000000" "0.000000, 0,90.000000" "1.000000,1.000000,1.000000")))
    (:NewEnumerator4
      (AddComponent|AddStaticMeshComponent false (Math|Transform|MakeTransform "0.000000,0.000000,-50.000000" "0.000000, 0,0.000000" "3.000000,3.000000,3.000000")))
    (:NewEnumerator5
      (AddComponent|AddStaticMeshComponent false (Math|Transform|ComposeTransforms (Math|Transform|MakeTransform "0.000000,0.000000,-50.000000" "0.000000, 0,0.000000" "2.762590,2.145767,0.994532") _returnvalue))
      (AddComponent|AddStaticMeshComponent false (Math|Transform|ComposeTransforms (Math|Transform|MakeTransform "0.000000,0.000000,-10.000000" "0.000000, 0,0.000000" "3.051758,2.441406,0.177979") _returnvalue)))))