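; RunningBackPawn_BP is a team-colored vehicle pawn with health.
; Forward input drives the movement component's throttle only in one specific RBGameState_BP state, and SetStop toggles the handbrake.
; Damage lowers health, and at zero or below the RBPlayerController_BP is told to respawn after a delay.
; The construction script reads the controller's player state team to apply a red or blue material to one mesh slot.
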(event Custom|SetStop
  (params (Stop :type Boolean))
  (Class|WheeledVehicleMovementComponent|SetHandbrakeInput (Variables|Default|GetVehicleMovement) Stop))

(event EventBeginPlay)

(event Collision|EventActorBeginOverlap
  (params (OtherActor :type Actor%20Object%20Reference)))

(event EventTick
  (params (DeltaSeconds :type Float%20%28single-precision%29)))

(event Game|Damage|EventAnyDamage
  (params (Damage :type Float%20%28single-precision%29) (DamageType :type Damage%20Type%20Object%20Reference) (InstigatedBy :type Controller%20Object%20Reference) (DamageCauser :type Actor%20Object%20Reference))
  (bind _output_get (Variables|Default|SetHealth (- (Variables|Default|GetHealth) Damage)))
  (if (<= _output_get 0.0)
    (bind _asrbplayer_controller_bp (Utilities|Casting|CastToRBPlayerController_BP (Pawn|GetController)))
    (Default|RespawnDelayed _asrbplayer_controller_bp)))

(event Input|AxisEvents|InputAxisMoveForward
  (params (AxisValue :type Float%20%28single-precision%29))
  (bind _asrbgame_state_bp (Utilities|Casting|CastToRBGameState_BP (Game|GetGameState)))
  (if (Utilities|Enum|Equal(Enum) (Variables|/Game/Blueprints/RBGameState_BP.RBGameState_BP_C|GetState _asrbgame_state_bp) "NewEnumerator5")
    (Class|WheeledVehicleMovementComponent|SetThrottleInput (Variables|Default|GetVehicleMovement) AxisValue)))

(fn ConstructionScript
  (bind _mesh (Variables|Character|GetMesh))
  (bind _asrbplayer_state_bp (Utilities|Casting|CastToRBPlayerState_BP (Variables|/Script/Engine.Controller|GetPlayerState (Pawn|GetController))))
  (switch Utilities|FlowControl|Switch|SwitchonETeam (Variables|/Script/RunningBack.RBPlayerState|GetTeam _asrbplayer_state_bp)
    (:VE_Red
      (Rendering|Material|SetMaterial _mesh 8 "/Game/Vehicle/RunningBack/red_texture.red_texture"))
    (:VE_Blue
      (Rendering|Material|SetMaterial _mesh 8 "/Game/Vehicle/RunningBack/blue_texture.blue_texture"))))