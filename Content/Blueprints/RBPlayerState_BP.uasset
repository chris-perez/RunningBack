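; RBPlayerState_BP is a player state that holds a player's points, team and running-back flag.
; ScorePoint increments Points, then has RBGameState_BP update the score and RBGameMode_BP check for a win.
; ChangeTeam calls SetTeam, which stores the team and tells the game state to update teams, while ChangeIsRunningBack only stores the flag.
; These changes print on-screen debug messages.
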(event Custom|ChangeIsRunningBack
  (params (IsRunningBack :type Boolean))
  (Development|PrintString "Change Is Running Back" true true "(R=0.000000,G=0.660000,B=1.000000,A=1.000000)" 1e+01)
  (bind _output_get (Variables|Default|SetIsRunningBack IsRunningBack))
  (Development|PrintString (Utilities|String|Append (Utilities|GetDisplayName (Game|GetPlayerController 0)) " (IsRunningBack): " (Utilities|String|ToString(Boolean) _output_get)) true true "(R=1.000000,G=0.616213,B=0.000000,A=1.000000)" 1e+01))

(event Custom|Change%20Team
  (params (Team :type ETeam%20Enum))
  (Development|PrintString "Change Team" true true "(R=1.000000,G=0.082433,B=0.000000,A=1.000000)" 1e+01)
  (CallFunction|SetTeam Team))

(event Custom|ScorePoint
  (bind _points (Variables|Default|GetPoints))
  (Math|Integer|IncrementInt _points
    (:%20%20
      (bind _asrbgame_state_bp (Utilities|Casting|CastToRBGameState_BP (Game|GetGameState)))
      (Default|UpdateScore _asrbgame_state_bp)
      (bind _asrbgame_mode_bp (Utilities|Casting|CastToRBGameMode_BP (Game|GetGameMode)))
      (Default|CheckWin _asrbgame_mode_bp)
      (Development|PrintString (Utilities|String|ToString(Integer) _points) true true "(R=1.000000,G=0.948292,B=0.331494,A=1.000000)" 5.0))))

(event EventBeginPlay)

(event EventTick
  (params (DeltaSeconds :type Float%20%28single-precision%29)))

(fn ConstructionScript)

(fn SetTeam
  (params (Team :type ETeam%20Enum))
  (Development|PrintString "Set Team" true true "(R=0.000000,G=0.660000,B=1.000000,A=1.000000)" 1e+01)
  (Variables|Default|SetTeam Team)
  (bind _asrbgame_state_bp (Utilities|Casting|CastToRBGameState_BP (Game|GetGameState)))
  (Default|UpdateTeams _asrbgame_state_bp))