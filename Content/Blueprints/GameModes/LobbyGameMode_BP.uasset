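; Lobby game mode that places joining players on Red or Blue and launches the multiplayer match.
; On PostLogin it puts the newcomer on Blue if Red has more players in the game state, otherwise Red, via the player state.
; It then has that player's controller show and refresh the lobby widget.
; StartGame clears widgets through the game state and server-travels to the aircraft carrier level under RBGameMode_BP.
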(event Custom|StartGame
  (bind _asrbgame_state_bp (Utilities|Casting|CastToRBGameState_BP (Game|GetGameState)))
  (Default|ClearWidgets _asrbgame_state_bp)
  (Class|LobbyGameMode|MyServerTravel "AircraftCarrier_Level_Multiplayer" "RBGameMode_BP" false))

(event EventPostLogin
  (params (NewPlayer :type Player%20Controller%20Object%20Reference))
  (bind _playerstate (Variables|/Script/Engine.Controller|GetPlayerState NewPlayer))
  ;[1 1 1] Chose what team the new player should be on
  (bind _asrbgame_state_bp (Utilities|Casting|CastToRBGameState_BP (Game|GetGameState)))
  (if (> (Utilities|Array|Length (Variables|/Game/Blueprints/RBGameState_BP.RBGameState_BP_C|GetRedTeam _asrbgame_state_bp)) (Utilities|Array|Length (Variables|/Game/Blueprints/RBGameState_BP.RBGameState_BP_C|GetBlueTeam _asrbgame_state_bp)))
    (bind _asrbplayer_state_bp (Utilities|Casting|CastToRBPlayerState_BP _playerstate))
    (Default|SetTeam _asrbplayer_state_bp "VE_Blue")
    (else
      (bind _asrbplayer_state_bp_2 (Utilities|Casting|CastToRBPlayerState_BP _playerstate))
      (Default|SetTeam _asrbplayer_state_bp_2 "VE_Red")))
  (bind _asrbplayer_controller (Utilities|Casting|CastToRBPlayerController NewPlayer))
  (Default|DisplayLobbyWidget _asrbplayer_controller)
  (Default|UpdateLobbyWidget _asrbplayer_controller)
  (Development|PrintString "Connected"))

(event EventBeginPlay)

(event EventTick
  (params (DeltaSeconds :type Float%20%28single-precision%29)))

(fn ConstructionScript)