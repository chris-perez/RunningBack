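; Game mode for a red-versus-blue running back match that starts play, handles scoring and ends the game.
; BeginPlay has RBGameState_BP assign running backs and count down, while PostLogin restores each player's state and updates teams.
; ScorePoint ends the game once either team exceeds MaxScore, showing a win screen to player 0 only.
; ChoosePlayerStart uses GetSpawn to pick a random team start, leaving an unused inline copy.
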(event Custom|ScorePoint
  (params (Player :type RB%20Player%20State%20Object%20Reference))
  (bind _max_score (Variables|Default|GetMax%20Score))
  ;[1 1 1] Score Point
  (Default|ScorePoint Player)
  (bind _asrbgame_state_bp (Utilities|Casting|CastToRBGameState_BP (Game|GetGameState)))
  (if (or (> (Variables|/Game/Blueprints/RBGameState_BP.RBGameState_BP_C|GetBlueScore _asrbgame_state_bp) _max_score) (> (Variables|/Game/Blueprints/RBGameState_BP.RBGameState_BP_C|GetRedScore _asrbgame_state_bp) _max_score))
    (CallFunction|EndGame)))

(event Custom|EndGame
  (bind _returnvalue (Game|GetPlayerController 0))
  ;[1 1 1] End Game
  (bind _returnvalue_2 (UserInterface|CreateWidget "/Game/UI/WinScreen.WinScreen_C" _returnvalue))
  (Input|SetInputModeUIOnly _returnvalue _returnvalue_2 false)
  (UserInterface|Viewport|AddtoViewport _returnvalue_2 0))

(event EventPostLogin
  (params (NewPlayer :type Player%20Controller%20Object%20Reference))
  ;[1 1 1] User Joins Session
  (Input|SetInputModeGameOnly NewPlayer)
  (bind _asrbplayer_controller (Utilities|Casting|CastToRBPlayerController NewPlayer))
  (Default|RestorePlayerState _asrbplayer_controller)
  (bind _asrbgame_state_bp (Utilities|Casting|CastToRBGameState_BP (Game|GetGameState)))
  (Default|UpdateTeams _asrbgame_state_bp))

(event EventBeginPlay
  (bind _returnvalue (Game|GetGameState))
  (bind _asrbgame_state_bp (Utilities|Casting|CastToRBGameState_BP _returnvalue))
  (Variables|/Game/Blueprints/RBGameState_BP.RBGameState_BP_C|SetStarted _asrbgame_state_bp true)
  (bind _asrbgame_state_bp_2 (Utilities|Casting|CastToRBGameState_BP _returnvalue))
  (Default|AssignRunningBacks _asrbgame_state_bp_2)
  (Default|Countdown _asrbgame_state_bp_2))

(event EventTick
  (params (DeltaSeconds :type Float%20%28single-precision%29)))

(fn ConstructionScript)

(fn ChoosePlayerStart
  (params (Player :type Controller%20Object%20Reference))
  (bind _returnvalue (Utilities|Casting|CastToPlayerController Player))
  (bind _returnvalue_2 (CallFunction|GetSpawn _returnvalue))
  (return _returnvalue_2))

(fn GetSpawn
  (params (Player :type Player%20Controller%20Object%20Reference))
  (bind _redspawns (Variables|Default|GetRedSpawns))
  (bind _bluespawns (Variables|Default|GetBlueSpawns))
  ;[1 1 1] Get player spawns by team and add them to arrays
  (Utilities|Array|Clear (Variables|Default|GetRedSpawns))
  (Utilities|Array|Clear (Variables|Default|GetBlueSpawns))
  (bind _outactors (Actor|GetAllActorsOfClass "/Game/Blueprints/TeamPlayerStart.TeamPlayerStart_C"))
  (for _array_element _outactors
    (if (Utilities|Enum|Equal(Enum) (Variables|/Game/Blueprints/TeamPlayerStart.TeamPlayerStart_C|GetTeam _array_element) "NewEnumerator0")
      (Utilities|Array|Add (Variables|Default|GetRedSpawns) _array_element)
      (else
        (Utilities|Array|Add (Variables|Default|GetBlueSpawns) _array_element))))
  (bind _asrbplayer_state (Utilities|Casting|CastToRBPlayerState (Variables|/Script/Engine.Controller|GetPlayerState Player)))
  (if (Utilities|Enum|Equal(Enum) (Variables|/Game/Blueprints/RBPlayerState.RBPlayerState_C|GetTeam _asrbplayer_state) "NewEnumerator0")
    (return (Utilities|Array|Get(acopy) _redspawns (Math|Random|RandomIntegerinRange 0 (- (Utilities|Array|Length _redspawns) 1))))
    (else
      (return (Utilities|Array|Get(acopy) _bluespawns (Math|Random|RandomIntegerinRange 0 (- (Utilities|Array|Length _bluespawns) 1)))))))