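; GameMode_BP is a game mode Blueprint that sets up the vehicle HUD and the pause menu.
; On BeginPlay it creates the VehicleHUD widget and adds it to the viewport.
; Pressing P creates a new PauseMenu widget, shows it, switches the player controller to UI-only input focused on it and pauses the game.
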(event EventBeginPlay
  (bind _output_get (Variables|Default|SetHUDWidgetClass "/Game/Blueprints/VehicleHUD.VehicleHUD_C"))
  (bind _returnvalue (UserInterface|CreateWidget _output_get))
  (UserInterface|Viewport|AddtoViewport _returnvalue 0))

(event EventTick
  (params (DeltaSeconds :type Float%20%28single-precision%29)))

(event Input|KeyboardEvents|P
  (params (Key :type Key%20Structure :default "AnyKey"))
  (:Pressed
    (bind _output_get (Variables|Default|SetPauseMenu "/Game/VehicleCPP/UI/PauseMenu.PauseMenu_C"))
    (bind _returnvalue (UserInterface|CreateWidget _output_get))
    (UserInterface|Viewport|AddtoViewport _returnvalue 0)
    (Input|SetInputModeUIOnly (Game|GetPlayerController 0) _returnvalue false)
    (Game|SetGamePaused true)))

(fn ConstructionScript
  (Variables|Default|SetPauseMenu "/Game/VehicleCPP/UI/PauseMenu.PauseMenu_C"))