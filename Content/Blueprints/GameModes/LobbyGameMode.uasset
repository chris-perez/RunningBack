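; Lobby game mode that assigns each joining player to a team, apparently to keep Red and Blue balanced.
; On PostLogin it compares the RedTeam and BlueTeam array lengths from RBGameState_BP.
; It then calls SetTeam on the player's RBPlayerState with one of two team enum values, treating a tie the same as Red having fewer players.
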(event EventPostLogin
  (params (NewPlayer :type Player%20Controller%20Object%20Reference))
  (bind _playerstate (Variables|/Script/Engine.Controller|GetPlayerState NewPlayer))
  ;[1 1 1] Chose what team the new player should be on
  (bind _asrbgame_state_bp (Utilities|Casting|CastToRBGameState_BP (Game|GetGameState)))
  (if (> (Utilities|Array|Length (Variables|/Game/Blueprints/RBGameState_BP.RBGameState_BP_C|GetRedTeam _asrbgame_state_bp)) (Utilities|Array|Length (Variables|/Game/Blueprints/RBGameState_BP.RBGameState_BP_C|GetBlueTeam _asrbgame_state_bp)))
    (bind _asrbplayer_state (Utilities|Casting|CastToRBPlayerState _playerstate))
    (Default|SetTeam _asrbplayer_state "NewEnumerator1")
    (else
      (bind _asrbplayer_state_2 (Utilities|Casting|CastToRBPlayerState _playerstate))
      (Default|SetTeam _asrbplayer_state_2 "NewEnumerator0"))))

(event EventBeginPlay)

(event EventTick
  (params (DeltaSeconds :type Float%20%28single-precision%29)))

(fn ConstructionScript)