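; Player state Blueprint that holds a player's points and team assignment.
; ScorePoint increments Points, then calls UpdateScore on RBGameState_BP.
; ChangeTeam stores the new team, then passes this player state to the game state's UpdateTeam.
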(event Custom|ScorePoint
  (bind _result (Math|Integer|IncrementInt (Variables|Default|GetPoints))
    (:%20%20
      (bind _asrbgame_state_bp (Utilities|Casting|CastToRBGameState_BP (Game|GetGameState)))
      (Default|UpdateScore _asrbgame_state_bp))))

(event EventBeginPlay)

(event EventTick
  (params (DeltaSeconds :type Float%20%28single-precision%29)))

(fn ConstructionScript)

(fn ChangeTeam
  (params (Team :type Team%20Enum))
  (Variables|Default|SetTeam Team)
  (bind _asrbgame_state_bp (Utilities|Casting|CastToRBGameState_BP (Game|GetGameState)))
  (Default|UpdateTeam _asrbgame_state_bp self))