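; AI controller, apparently for a running back pawn, that hands movement to the BackAndForth behavior tree.
; On BeginPlay it seeds AIBlackboard with HomeLocation, the pawn's location with X and Y doubled, and a TargetLocation offset from that along X.
; It prints both points for debugging, then runs the tree.
; Unconnected experiments with vehicle throttle and several move-to nodes remain in the graph but never run.
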(event EventBeginPlay
  (bind _returnvalue (Pawn|GetControlledPawn))
  (bind _self self)
  (bind _homelocation (Variables|Default|GetHomeLocation))
  (bind _targetlocation (Variables|Default|GetTargetLocation))
  (bind _returnvalue_2 (AI|GetBlackboard _self))
  (bind _returnvalue_3 (Transformation|GetActorLocation _returnvalue))
  (bind _returnvalue_4 (* _returnvalue_3 "2.000000,2.000000,1.000000"))
  (Class|AIController|UseBlackboard "/Game/Blueprints/AI/AIBlackboard.AIBlackboard")
  (AI|Components|Blackboard|SetValueasVector _returnvalue_2 _homelocation _returnvalue_4)
  (AI|Components|Blackboard|SetValueasVector _returnvalue_2 _targetlocation (+ _returnvalue_4 "5000.000000, 0, 0"))
  (Development|PrintString (Utilities|String|Append "Home Loccation" (Utilities|String|ToString(Vector) (AI|Components|Blackboard|GetValueasVector _returnvalue_2 _homelocation))) true true "(R=0.000000,G=0.660000,B=1.000000,A=1.000000)" 5.0)
  (Development|PrintString (Utilities|String|Append "TargetLoccation" (Utilities|String|ToString(Vector) (AI|Components|Blackboard|GetValueasVector _returnvalue_2 _targetlocation))) true true "(R=0.000000,G=0.660000,B=1.000000,A=1.000000)" 5.0)
  (AI|RunBehaviorTree "/Game/Blueprints/AI/BackAndForth.BackAndForth"))

(event EventTick
  (params (DeltaSeconds :type Float%20%28single-precision%29)))

(fn ConstructionScript)