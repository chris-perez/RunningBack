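; Behavior tree task that moves an RBAIControllerNew's pawn straight to the TargetLocation blackboard vector, with pathfinding disabled.
; A target Z at or below -1000 is replaced by the pawn's nav agent height before AIMoveTo runs.
; Request Failed finishes the task as success and Move Finished as failure, opposite to the pin names, both printing debug text.
; Alternative move, cast and trace experiments remain as unconnected nodes.
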(event EventReceiveExecute
  (params (OwnerActor :type Actor%20Object%20Reference))
  (bind _targetlocation (Variables|Default|GetTargetLocation))
  (bind _returnvalue (Class|BTFunctionLibrary|GetBlackboardValueasVector _targetlocation))
  (bind (_x _y _z) (Math|Vector|BreakVector _returnvalue))
  (if (!= 0 0)
    _
    (else
      _))
  (bind _asrbaicontroller_new (Utilities|Casting|CastToRBAIControllerNew OwnerActor))
  (Variables|Default|SetAI_CON_Ref _asrbaicontroller_new)
  (AI|AIMoveTo (Variables|Default|GetAI_CON_Ref) (select (<= _z -1e+03) (Math|Vector|MakeVector _x _y (.Z (Math|Vector|BreakVector (Pawn|GetNavAgentLocation (Pawn|GetControlledPawn (Variables|Default|GetAI_CON_Ref)))))) _returnvalue) 0 1e+02 "Default" "Disable" false true
    (:OnRequestFailed
      (AI|BehaviorTree|FinishExecute true)
      (Development|PrintString "AI Move To Success" true true "(R=0.000000,G=1.000000,B=0.051749,A=1.000000)"))
    (:OnMoveFinished
      (AI|BehaviorTree|FinishExecute false)
      (Development|PrintString "AI Move To Failed" true true "(R=1.000000,G=0.077341,B=0.144250,A=1.000000)")))
  (Development|PrintString (Utilities|String|ToString(Vector) (select (<= _z -1e+03) (Math|Vector|MakeVector _x _y (.Z (Math|Vector|BreakVector (Pawn|GetNavAgentLocation (Pawn|GetControlledPawn (Variables|Default|GetAI_CON_Ref)))))) _returnvalue)))
  (Development|PrintString "Hello" true true "(R=1.000000,G=0.000000,B=0.077258,A=1.000000)"))