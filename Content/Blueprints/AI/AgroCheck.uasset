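; Behavior tree service that looks for targets around the AI pawn for aggro and writes them to the blackboard.
; Each tick it sphere-traces for desired object types through the cached RBAIController_BP's pawn, ignoring all AIPawns, then line-traces to each hit on the Camera channel.
; A clear line sets TargetToFollow and TargetLocation; otherwise TargetToFollow receives the line-trace result, whose name is printed.
; Both traces draw debug shapes.
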(event EventReceiveTickAI
  (params (OwnerController :type AI%20Controller%20Object%20Reference) (ControlledPawn :type Pawn%20Object%20Reference) (DeltaSeconds :type Float%20%28single-precision%29))
  ;[1 1 1] Is AI_CON_Ref set?
  (if (!= (Variables|Default|GetAI_CON_Ref) 0)
    _
    (else
      (bind _asrbaicontroller_bp (Utilities|Casting|CastToRBAIController_BP OwnerController))
      (Variables|Default|SetAI_CON_Ref _asrbaicontroller_bp)))
  (bind _outactors (Actor|GetAllActorsOfClass "/Game/Blueprints/AI/AIPawn.AIPawn_C"))
  (Variables|Default|SetMyLocation (Transformation|GetActorLocation (Pawn|GetControlledPawn (Variables|Default|GetAI_CON_Ref))))
  (bind _outhits (Collision|MultiSphereTraceForObjects (Transformation|GetActorLocation (Pawn|GetControlledPawn (Variables|Default|GetAI_CON_Ref))) (+ (Transformation|GetActorLocation (Pawn|GetControlledPawn (Variables|Default|GetAI_CON_Ref))) "0,0.000000,15.000000") 3e+03 (Variables|Default|GetDesiredObjectTypes) false _outactors "ForDuration"))
  (bind _array_element (Utilities|Array|ForEachLoopwithBreak _outhits)
    (:LoopBody
      (bind _outhit (Collision|LineTraceByChannel (Variables|Default|GetMyLocation) (Transformation|GetActorLocation (.HitActor (Collision|BreakHitResult _array_element))) "TraceTypeQuery2" false _outactors "ForDuration"))
      (if (== (.HitActor (Collision|BreakHitResult _outhit)) (.HitActor (Collision|BreakHitResult _array_element)))
        (Class|BTFunctionLibrary|SetBlackboardValueasObject (Variables|Default|GetTargetToFollow) (.HitActor (Collision|BreakHitResult _outhit)))
        (AI|BehaviorTree|SetBlackboardValueasVector (Variables|Default|GetTargetLocation) (Transformation|GetActorLocation (.HitActor (Collision|BreakHitResult _outhit))))
        (else
          (Class|BTFunctionLibrary|SetBlackboardValueasObject (Variables|Default|GetTargetToFollow) (.HitActor (Collision|BreakHitResult _outhit)))
          (Development|PrintString (Utilities|GetDisplayName (.HitActor (Collision|BreakHitResult _outhit))) true true "(R=0.284948,G=0.429935,B=1.000000,A=1.000000)"))))))