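; Behavior tree decorator that checks whether the AI's controlled pawn is close enough to a target location.
; It casts the owner to RBAIController_BP, caches that reference, and reads the target vector from the blackboard.
; The condition passes when the straight-line 3D distance from the pawn to the target is within AcceptableDistance.
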(fn PerformConditionCheck
  (params (OwnerActor :type Actor%20Object%20Reference))
  (bind _asrbaicontroller_bp (Utilities|Casting|CastToRBAIController_BP OwnerActor))
  (Variables|Default|SetAI_CON_Ref _asrbaicontroller_bp)
  (return (<= (Math|Vector|VectorLength (- (Class|BTFunctionLibrary|GetBlackboardValueasVector (Variables|Default|GetTargetLocation)) (Transformation|GetActorLocation (Pawn|GetControlledPawn (Variables|Default|GetAI_CON_Ref))))) (Variables|Default|GetAcceptableDistance))))