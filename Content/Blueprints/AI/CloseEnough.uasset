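; CloseEnough is an AI condition check, in the form of a Behavior Tree decorator, that currently always returns false.
; PerformConditionCheck casts the owner to RBAIController_BP and caches it in AICONRef before returning.
; An unconnected expression compares the distance between the controlled pawn and the TargetToFollow blackboard actor with AcceptableDistance, testing for at least that distance, but it does not affect the result.
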(fn PerformConditionCheck
  (params (OwnerActor :type Actor%20Object%20Reference))
  (bind _asrbaicontroller_bp (Utilities|Casting|CastToRBAIController_BP OwnerActor))
  (Variables|Default|SetAI_CON_Ref _asrbaicontroller_bp)
  (return false))