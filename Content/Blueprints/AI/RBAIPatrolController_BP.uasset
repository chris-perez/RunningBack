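; AI controller that runs a patrol behavior tree for its controlled pawn.
; On BeginPlay it sets up the AI blackboard and starts the Patrol tree, leaving movement logic to that tree.
; Unconnected leftover experiments remain in the graph: throttle input on a RunningBackPawn, several move-to methods along +Y, and seeding Home and Target blackboard locations with debug prints.
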(event EventBeginPlay
  (Class|AIController|UseBlackboard "/Game/Blueprints/AI/AIBlackboard.AIBlackboard")
  (AI|RunBehaviorTree "/Game/Blueprints/AI/Patrol.Patrol"))

(event EventTick
  (params (DeltaSeconds :type Float%20%28single-precision%29)))

(fn ConstructionScript)