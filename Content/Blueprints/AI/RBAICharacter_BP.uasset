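; RBAICharacter_BP is an AI character Blueprint that displays a health bar for its life points.
; Each Tick casts the widget component's user widget to HealthBar and sets its progress bar to LifePoints over MaxLifePoints.
; It then yaws the HealthBarScene component toward the pawn controlled by player 0, with pitch and roll held at zero so the bar stays upright.
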(event EventBeginPlay)

(event EventActorBeginOverlap
  (params (OtherActor :type Actor%20Object%20Reference)))

(event EventTick
  (params (DeltaSeconds :type Float%20%28single-precision%29))
  (bind _healthbarscene (Variables|Default|GetHealthBarScene))
  (bind _ashealth_bar (Utilities|Casting|CastToHealthBar (UserInterface|GetUserWidgetObject (Variables|Default|GetHealthBar))))
  (Progress|SetPercent (Variables|/Game/UI/HealthBar.HealthBar_C|GetHealth _ashealth_bar) (/ (Variables|Default|GetLifePoints) (Variables|Default|GetMaxLifePoints)))
  (Transformation|SetWorldRotation _healthbarscene (Math|Rotator|MakeRotator 0.0 0.0 (.Yaw (Math|Rotator|BreakRotator (Math|Rotator|FindLookatRotation (Transformation|GetWorldLocation _healthbarscene) (Transformation|GetActorLocation (Pawn|GetControlledPawn (Game|GetPlayerController 0))))))) false false))

(fn ConstructionScript)