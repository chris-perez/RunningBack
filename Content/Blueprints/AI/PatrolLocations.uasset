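; Behavior tree task that advances an RBAIPatrolController_BP's patrol target to the next point in its PatrolLocations array.
; It finds the current TargetLocation blackboard vector in the array and writes the following entry, wrapping to the first at the end.
; It then prints a debug message and finishes successfully without moving the pawn.
; An AI MoveTo branch toward TargetToFollow is left disconnected and never runs.
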(event EventReceiveExecute
  (params (OwnerActor :type Actor%20Object%20Reference))
  (bind _targetlocation (Variables|Default|GetTargetLocation))
  (if (!= (Variables|Default|GetAI_CON_Ref) 0)
    _
    (else
      _))
  (bind _asrbaipatrol_controller_bp (Utilities|Casting|CastToRBAIPatrolController_BP OwnerActor))
  (bind _output_get (Variables|Default|SetAI_CON_Ref _asrbaipatrol_controller_bp))
  (if (>= (+ (Utilities|Array|FindItem (Variables|/Game/Blueprints/AI/RBAIPatrolController_BP.RBAIPatrolController_BP_C|GetPatrolLocations _output_get) (AI|Components|Blackboard|GetValueasVector (AI|GetBlackboard _output_get) _targetlocation)) 1) 0)
    (if (>= (+ (Utilities|Array|FindItem (Variables|/Game/Blueprints/AI/RBAIPatrolController_BP.RBAIPatrolController_BP_C|GetPatrolLocations _output_get) (AI|Components|Blackboard|GetValueasVector (AI|GetBlackboard _output_get) _targetlocation)) 1) (Utilities|Array|Length (Variables|/Game/Blueprints/AI/RBAIPatrolController_BP.RBAIPatrolController_BP_C|GetPatrolLocations _output_get)))
      (AI|Components|Blackboard|SetValueasVector (AI|GetBlackboard _output_get) _targetlocation (Utilities|Array|Get(acopy) (Variables|/Game/Blueprints/AI/RBAIPatrolController_BP.RBAIPatrolController_BP_C|GetPatrolLocations _output_get)) :!label _label)
      (else
        (AI|Components|Blackboard|SetValueasVector (AI|GetBlackboard _output_get) _targetlocation (Utilities|Array|Get(acopy) (Variables|/Game/Blueprints/AI/RBAIPatrolController_BP.RBAIPatrolController_BP_C|GetPatrolLocations _output_get) (+ (Utilities|Array|FindItem (Variables|/Game/Blueprints/AI/RBAIPatrolController_BP.RBAIPatrolController_BP_C|GetPatrolLocations _output_get) (AI|Components|Blackboard|GetValueasVector (AI|GetBlackboard _output_get) _targetlocation)) 1)))))
    (else
      (goto _label)))
  (Development|PrintString (Utilities|String|Append "TargetLocation: " (Utilities|String|ToString(Vector) (Utilities|Array|Get(acopy) (Variables|/Game/Blueprints/AI/RBAIPatrolController_BP.RBAIPatrolController_BP_C|GetPatrolLocations _output_get) (+ (Utilities|Array|FindItem (Variables|/Game/Blueprints/AI/RBAIPatrolController_BP.RBAIPatrolController_BP_C|GetPatrolLocations _output_get) (AI|Components|Blackboard|GetValueasVector (AI|GetBlackboard _output_get) _targetlocation)) 1)))) true true "(R=0.000000,G=1.000000,B=0.478753,A=1.000000)" 5.0)
  (AI|BehaviorTree|FinishExecute true))