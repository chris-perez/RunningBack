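; Behavior tree task that moves an RBAIController_BP's pawn to the TargetToFollow blackboard actor.
; On execute, only while AICONRef is unset, it caches the controller and runs AI Move To with a tight acceptance radius.
; Results are inverted: a successful move finishes the task as failed, and a failed move finishes it as succeeded.
; Both outcomes print debug text, with failure adding target name, location and movement result.
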(event EventReceiveExecute
  (params (OwnerActor :type Actor%20Object%20Reference))
  (bind _targettofollow (Variables|Default|GetTargetToFollow))
  (bind _returnvalue (AI|BehaviorTree|GetBlackboardValueasActor _targettofollow))
  (if (not (!= (Variables|Default|GetAI_CON_Ref) 0))
    (bind _asrbaicontroller_bp (Utilities|Casting|CastToRBAIController_BP OwnerActor))
    (Variables|Default|SetAI_CON_Ref _asrbaicontroller_bp)
    (bind _movementresult (AI|AIMoveTo (Pawn|GetControlledPawn (Variables|Default|GetAI_CON_Ref)) "0, 0, 0" _returnvalue 1e+01 true)
      (:OnSuccess
        (AI|BehaviorTree|FinishExecute false)
        (Development|PrintString "AI Move To Success" true true "(R=0.000000,G=1.000000,B=0.051749,A=1.000000)"))
      (:OnFail
        (Development|PrintString "AI Move To Failed")
        (Development|PrintString (Utilities|GetDisplayName _returnvalue))
        (Development|PrintString (Utilities|String|ToString(Vector) (+ (Transformation|GetActorLocation _returnvalue) "0.000000,0.000000,0.000000")))
        (Development|PrintString (Utilities|String|EnumtoString _movementresult))
        (AI|BehaviorTree|FinishExecute true)))))