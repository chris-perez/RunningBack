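; AI controller Blueprint that runs a simple move test on its controlled pawn.
; One second after BeginPlay, an async AI MoveTo sends the pawn to a point diagonally offset from its current location.
; Print strings report the task object's name and whether the move succeeds or fails.
; A blackboard and behavior tree setup that stores the pawn's location as HomeLocation is left disconnected and never runs.
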(event EventBeginPlay
  (Utilities|FlowControl|Delay 1.0)
  (bind _asynctaskproxy (AI|AIMoveTo self (+ (Transformation|GetActorLocation (Pawn|GetControlledPawn)) "100.000000,100.000000, 0") 0 -1.0 "Default" "Default" true true)
    (:then
      (Development|PrintString (Utilities|GetDisplayName _asynctaskproxy)))
    (:OnRequestFailed
      (Development|PrintString "Move Failed"))
    (:OnMoveFinished
      (Development|PrintString "Move Succeeded"))))

(event EventTick
  (params (DeltaSeconds :type Float%20%28single-precision%29)))

(fn ConstructionScript)