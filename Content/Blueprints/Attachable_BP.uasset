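; Attachable Blueprint that displays the weapon mesh stored in the game instance.
; On BeginPlay it casts the game instance to RBGameInstance and checks the DefaultChanged flag.
; When the flag is set, it applies the saved AttachedGun mesh, scale, relative location and rotation to its Weapon component; otherwise the component keeps its defaults.
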(event EventBeginPlay
  (bind _weapon (Variables|Default|GetWeapon))
  (bind _asrbgame_instance (Utilities|Casting|CastToRBGameInstance (Game|GetGameInstance)))
  (if (Variables|/Game/Blueprints/RBGameInstance.RBGameInstance_C|GetDefaultChanged _asrbgame_instance)
    (Components|StaticMesh|SetStaticMesh _weapon (Variables|/Game/Blueprints/RBGameInstance.RBGameInstance_C|GetAttachedGun _asrbgame_instance))
    (Transformation|SetRelativeScale3D _weapon (Variables|/Game/Blueprints/RBGameInstance.RBGameInstance_C|GetScale _asrbgame_instance))
    (Transformation|SetRelativeLocationAndRotation _weapon (Variables|/Game/Blueprints/RBGameInstance.RBGameInstance_C|GetLocation _asrbgame_instance) (Variables|/Game/Blueprints/RBGameInstance.RBGameInstance_C|GetRotation _asrbgame_instance) false false)))

(event EventActorBeginOverlap
  (params (OtherActor :type Actor%20Object%20Reference)))

(event EventTick
  (params (DeltaSeconds :type Float%20%28single-precision%29)))

(fn ConstructionScript)