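; Endzone actor that awards a point when an opposing team's running back enters it.
; On overlap it resolves the pawn's RBPlayerController and RBPlayerState, checks the running back role and team, then calls ScorePoint on RBGameMode.
; The construction script colors the cube with the red or blue endzone material based on its Team setting.
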(event EventBeginPlay)

(event EventActorBeginOverlap
  (params (OtherActor :type Actor%20Object%20Reference))
  (bind _asrunning_back_pawn_bp (Utilities|Casting|CastToRunningBackPawn_BP OtherActor))
  (bind _asrbplayer_controller (Utilities|Casting|CastToRBPlayerController (Pawn|GetController _asrunning_back_pawn_bp)))
  (bind _asrbplayer_state (Utilities|Casting|CastToRBPlayerState (Variables|/Script/Engine.Controller|GetPlayerState _asrbplayer_controller)))
  (if (Variables|/Game/Blueprints/RBPlayerState.RBPlayerState_C|GetIsRunningBack _asrbplayer_state)
    (if (not (Utilities|Enum|Equal(Enum) (Variables|/Game/Blueprints/RBPlayerState.RBPlayerState_C|GetTeam _asrbplayer_state) (Variables|Default|GetTeam)))
      (bind _asrbgame_mode (Utilities|Casting|CastToRBGameMode (Game|GetGameMode)))
      (Default|ScorePoint _asrbgame_mode _asrbplayer_state))))

(event EventTick
  (params (DeltaSeconds :type Float%20%28single-precision%29)))

(fn ConstructionScript
  (bind _cube (Variables|Default|GetCube))
  (if (Utilities|Enum|Equal(Enum) (Variables|Default|GetTeam) "NewEnumerator0")
    (Rendering|Material|SetMaterial _cube 0 "/Game/RedEndzone.RedEndzone")
    (else
      (Rendering|Material|SetMaterial _cube 0 "/Game/BlueEndzone.BlueEndzone"))))